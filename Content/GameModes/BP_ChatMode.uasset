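; BP_ChatMode is a game mode Blueprint for a chat-based Bulls and Cows number-guessing game, currently left as an unwired draft.
; GotMessageFromClient receives a message and player ID but does nothing.
; Disconnected fragments validate three-digit guesses, broadcast messages to every BP_Controller and print a test of random answer generation and scoring.
; An unused expression checks host versus client turn from PlayerId and IsHostTurn.
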(event `GotMessageFromClient`
  (params (Msg :type String) (PlayerId :type Integer)))

(fn `UserConstructionScript`)