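; BP_Controller is a chat controller with events for login, receiving broadcasts and sending messages, but all its events are empty.
; Disconnected logic would store the user ID, bind to the chat window widget after a delay and add received text to the HUD.
; Another unwired chain would pass ID-prefixed messages and the player ID to BP_ChatMode, the game mode.
; None of this logic runs as wired.
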(event `self.ReceiveBeginPlay`)

(event `OnLoginWithID`
  (params (UserId :type String)))

(event `GotBroadcast`
  (params (Msg :type String)))

(event `OnSendMsgToServer`
  (params (Msg :type String)))

(fn `UserConstructionScript`)